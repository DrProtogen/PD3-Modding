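; Function library for the PDML mod loader that turns each mod's metadata into SBZ settings menu categories and persists their values.
; CreateModSettings builds typed settings (toggle, float, color, keybind, string) into groups, preferring saved values over defaults, then registers the category in ModLoaderManager's ModSettingsConfig.
; Values live in per-category SaveGame slots, which every getter reloads and every setter reloads and rewrites.
; CreateGeneralCategory is an unfinished stub.
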(fn `CreateColorSetting`
  (params (UniqueName :type Name) (`Display Text` :type Text) (`Apply Change Immediately` :type Boolean) (`Get Default Value Function Name` :type Name) (`Get Value Function Name` :type Name) (`Set Value Function Name` :type Name) (`Color Value` :type "LinearColor Structure"))
  (returns (SBZSettingData :type "SBZSettingData Structure"))
  (return (make `SBZSettingData` `Display Text` false "" false "" UniqueName "" "ColorControl" "None" "" `Apply Change Immediately` false true "GetButtonVisibilityAlways" false false false "" "None" `Get Default Value Function Name` `Get Value Function Name` `Set Value Function Name` "GetDefaultPrimaryKeyboardBinding" "GetPrimaryKeyboardBinding" "SetPrimaryKeyboardBinding" "GetDefaultSecondaryKeyboardBinding" "GetSecondaryKeyboardBinding" "SetSecondaryKeyboardBinding" true true "" "" false false "" 0 0 0.0 0.0 0.0 0.0 0.0 "" "" `Color Value` `Color Value`)))

(fn `CreateFloatSetting`
  (params (UniqueName :type Name) (`Display Text` :type Text) (`Apply Change Immediately` :type Boolean) (`Get Default Value Function Name` :type Name) (`Get Value Function Name` :type Name) (`Set Value Function Name` :type Name) (`Float Min Value` :type "Float (double-precision)") (`Float Max Value` :type "Float (double-precision)") (`Float Increment Value` :type "Float (double-precision)") (`Float Value` :type "Float (double-precision)"))
  (returns (SBZSettingData :type "SBZSettingData Structure"))
  (return (make `SBZSettingData` `Display Text` false "" false "" UniqueName "" "Slider" "None" "" `Apply Change Immediately` false true "GetButtonVisibilityAlways" false false false "" "None" `Get Default Value Function Name` `Get Value Function Name` `Set Value Function Name` "GetDefaultPrimaryKeyboardBinding" "GetPrimaryKeyboardBinding" "SetPrimaryKeyboardBinding" "GetDefaultSecondaryKeyboardBinding" "GetSecondaryKeyboardBinding" "SetSecondaryKeyboardBinding" true true "" "" false false "" 0 0 `Float Min Value` `Float Max Value` `Float Increment Value` `Float Value` `Float Value`)))

(fn `CreateGeneralCategory`
  (locals (Settings :type "Array of SBZSettingData Structure") (CurrentBools :type "Array of Name"))
  (bind _categoryname (`self.GetCategoryNameFromModName` "General"))
  (bind _config (`self.LoadConfig` (`KismetStringLibrary.Conv_NameToString` _categoryname)))
  (bind _keys (`BlueprintMapLibrary.Map_Keys` (`/PDML/Blueprints/SaveGame/SaveGame_PDML_Settings.ToggleMap` _config)))
  (if (> (`KismetArrayLibrary.Array_Length` _keys) 0)
    _))

(fn `CreateKeybindSetting`
  (params (UniqueName :type Name) (`Display Text` :type Text) (`Apply Change Immediately` :type Boolean) (`Get Default Value Function Name` :type Name) (`Get Value Function Name` :type Name) (`Set Value Function Name` :type Name) (`Primary Binding` :type "InputChord Structure") (`Secondary Binding` :type "InputChord Structure"))
  (returns (SBZSettingData :type "SBZSettingData Structure"))
  (return (make `SBZSettingData` :`SettingNameLocalized` `Display Text` :`SettingName` UniqueName :`ControlType` "KeyboardInputBinding" :`bApplyChangeImmediately` `Apply Change Immediately` :`bCanResetToDefault` true :`GetButtonVisibilityFunctionName` "GetButtonVisibilityAlways" :`GetDefaultValueFunctionName` `Get Default Value Function Name` :`GetValueFunctionName` `Get Value Function Name` :`SetValueFunctionName` `Set Value Function Name` :`GetDefaultKeyPrimaryFunctionName` "GetDefaultPrimaryKeyboardBinding" :`GetKeyPrimaryFunctionName` "GetPrimaryKeyboardBinding" :`SetKeyPrimaryFunctionName` "SetPrimaryKeyboardBinding" :`GetDefaultKeySecondaryFunctionName` "GetDefaultSecondaryKeyboardBinding" :`GetKeySecondaryFunctionName` "GetSecondaryKeyboardBinding" :`SetKeySecondaryFunctionName` "SetSecondaryKeyboardBinding" :`ButtonVisibilityPrevious` true :`ButtonVisibilityCurrent` true :`PrimaryBinding` `Primary Binding` :`SecondaryBinding` `Secondary Binding`)))

(fn `CreateModSettings`
  (params (ModMeta :type "/PDML/Blueprints/PDA_ModMeta Object Reference"))
  (locals (Groups :type "Array of SBZSettingsMenuGroupInfo Structure") (CurrentSettings :type "Array of SBZSettingData Structure"))
  (bind _modid (`/PDML/Blueprints/PDA_ModMeta.ModID` ModMeta))
  (bind _groups (`local.Groups`))
  (`KismetArrayLibrary.Array_Clear` (`local.Groups`))
  (bind _categoryname (`self.GetCategoryNameFromModName` _modid))
  (bind _returnvalue (`KismetStringLibrary.Conv_NameToString` _categoryname))
  (bind (_config _firsttime) (`self.LoadConfig` _returnvalue))
  (for _array_element (`/PDML/Blueprints/PDA_ModMeta.Settings` ModMeta)
    (`KismetArrayLibrary.Array_Clear` (`local.CurrentSettings`))
    (`|ExecutionSequence`
      (:`then_0`
        (bind (_uniqueid _displaytext _togglesettings _floatsettings _colorsettings _keybindsettings _stringsettings) (break `/PDML/Blueprints/Settings/FPDML_Settings_Group` _array_element))
        (for _array_element_2 _togglesettings
          (bind (_uniqueid_2 _displaytext_2 _defaultvalue) (break `/PDML/Blueprints/Settings/FPDML_Settings_Bool` _array_element_2))
          (bind (_value _returnvalue_2) (`BlueprintMapLibrary.Map_Find` (`/PDML/Blueprints/SaveGame/SaveGame_PDML_Settings.ToggleMap` _config) _uniqueid_2))
          (bind _returnvalue_3 (select `bool` (or (== _returnvalue_2 false) _firsttime) :`false` _value :`true` _defaultvalue))
          (bind _sbzsettingdata (`self.CreateToggleSetting` _uniqueid_2 (`KismetTextLibrary.Conv_StringToText` _displaytext_2) true "None" "None" "None" _returnvalue_3))
          (`KismetArrayLibrary.Array_Add` (`local.CurrentSettings`) _sbzsettingdata)
          (`self.SetToggleSettingValue` _returnvalue _uniqueid_2 _returnvalue_3)))
      (:`then_1`
        (for _array_element_3 _floatsettings
          (bind (_uniqueid_3 _displaytext_3 _min _max _incrementvalue _defaultvalue_2) (break `/PDML/Blueprints/Settings/FPDML_Settings_Float` _array_element_3))
          (bind (_value_2 _returnvalue_4) (`BlueprintMapLibrary.Map_Find` (`/PDML/Blueprints/SaveGame/SaveGame_PDML_Settings.FloatMap` _config) _uniqueid_3))
          (bind _returnvalue_5 (`KismetMathLibrary.SelectFloat` _defaultvalue_2 _value_2 (or (== _returnvalue_4 false) _firsttime)))
          (bind _sbzsettingdata_2 (`self.CreateFloatSetting` _uniqueid_3 (`KismetTextLibrary.Conv_StringToText` _displaytext_3) true "None" "None" "None" _min _max _incrementvalue _returnvalue_5))
          (`KismetArrayLibrary.Array_Add` (`local.CurrentSettings`) _sbzsettingdata_2)
          (`self.SetFloatSettingValue` _returnvalue _uniqueid_3 _returnvalue_5)))
      (:`then_2`
        (for _array_element_4 _colorsettings
          (bind (_uniqueid_4 _displaytext_4 _defaultvalue_3) (break `/PDML/Blueprints/Settings/FPDML_Settings_Color` _array_element_4))
          (bind (_value_3 _returnvalue_6) (`BlueprintMapLibrary.Map_Find` (`/PDML/Blueprints/SaveGame/SaveGame_PDML_Settings.ColorMap` _config) _uniqueid_4))
          (bind _returnvalue_7 (`KismetMathLibrary.SelectColor` _defaultvalue_3 _value_3 (or (== _returnvalue_6 false) _firsttime)))
          (bind _sbzsettingdata_3 (`self.CreateColorSetting` _uniqueid_4 (`KismetTextLibrary.Conv_StringToText` _displaytext_4) true "None" "None" "None" _returnvalue_7))
          (`KismetArrayLibrary.Array_Add` (`local.CurrentSettings`) _sbzsettingdata_3)
          (`self.SetColorSettingValue` _returnvalue _uniqueid_4 _returnvalue_7)))
      (:`then_3`
        (for _array_element_5 _keybindsettings
          (bind (_uniqueid_5 _displaytext_5 _defaultprimary _defaultsecondary) (break `/PDML/Blueprints/Settings/FPDML_Settings_Keybind` _array_element_5))
          (bind (_value_4 _returnvalue_8) (`BlueprintMapLibrary.Map_Find` (`/PDML/Blueprints/SaveGame/SaveGame_PDML_Settings.PrimaryKeybindMap` _config) _uniqueid_5))
          (bind _returnvalue_9 (select `bool` (or (== _returnvalue_8 false) _firsttime) :`false` _value_4 :`true` _defaultprimary))
          (bind (_value_5 _returnvalue_10) (`BlueprintMapLibrary.Map_Find` (`/PDML/Blueprints/SaveGame/SaveGame_PDML_Settings.SecondaryKeybindMap` _config) _uniqueid_5))
          (bind _returnvalue_11 (select `bool` (or (== _returnvalue_10 false) _firsttime) :`false` _value_5 :`true` _defaultsecondary))
          (bind _sbzsettingdata_4 (`self.CreateKeybindSetting` _uniqueid_5 (`KismetTextLibrary.Conv_StringToText` _displaytext_5) true "None" "None" "None" _returnvalue_9 _returnvalue_11))
          (`KismetArrayLibrary.Array_Add` (`local.CurrentSettings`) _sbzsettingdata_4)
          (`self.SetKeybindSettingValue` _returnvalue _uniqueid_5 _returnvalue_9 _returnvalue_11)))
      (:`then_4`
        (for _array_element_6 _stringsettings
          (bind (_uniqueid_6 _displaytext_6 _value_6) (break `/PDML/Blueprints/Settings/FPDML_Settings_String` _array_element_6))
          (bind (_value_7 _returnvalue_12) (`BlueprintMapLibrary.Map_Find` (`/PDML/Blueprints/SaveGame/SaveGame_PDML_Settings.StringMap` _config) _uniqueid_6))
          (bind _returnvalue_13 (`KismetMathLibrary.SelectString` _value_6 _value_7 (or (== _returnvalue_12 false) _firsttime)))
          (bind _sbzsettingdata_5 (`self.CreateStringSetting` _uniqueid_6 (`KismetTextLibrary.Conv_StringToText` _displaytext_6) true "None" "None" "None" _returnvalue_13))
          (`KismetArrayLibrary.Array_Add` (`local.CurrentSettings`) _sbzsettingdata_5)
          (`self.SetStringSetting` _returnvalue _uniqueid_6 _returnvalue_13)))
      (:`then_5`
        (bind _array (`self.CreateSettingsGroup` _modid _uniqueid (`KismetStringLibrary.Conv_StringToName` _displaytext) (`local.CurrentSettings`)))
        (`KismetArrayLibrary.Array_Append` (`local.Groups`) _array))))
  (if (not (`KismetArrayLibrary.Array_IsEmpty` _groups))
    (`self.CreateSettingCategory` _modid _groups)))

(fn `CreateModSettingsAll`
  (params (ModMetas :type "Array of /PDML/Blueprints/PDA_ModMeta Object Reference"))
  (locals (CurrentSettings :type "Array of SBZSettingData Structure") (Groups :type "Array of SBZSettingsMenuGroupInfo Structure"))
  (`|ExecutionSequence`
    (:`then_0`
      (`self.CreateGeneralCategory` null))
    (:`then_1`
      (for _array_element ModMetas
        (`self.CreateModSettings` _array_element)))))

(fn `CreateSettingCategory`
  (params (ModName :type Name) (`Settings Groups` :type "Array of SBZSettingsMenuGroupInfo Structure"))
  (returns (Successful :type Boolean))
  (locals (bFound :type Boolean))
  (bind _categoryname (`self.GetCategoryNameFromModName` ModName))
  (bind _bexists (`self.DoesCategoryAlreadyExist` _categoryname))
  (if _bexists
    (`/PDML/Blueprints/Utilities/BPFL_ModLoader.PrintToModLoader` (`KismetTextLibrary.Conv_TextToString` (`|FormatText` "Failed to create {category} settings as it already exists! " _categoryname)))
    (return false)
    (else
      (`/PDML/Blueprints/Utilities/BPFL_ModLoader.PrintToModLoader` (`KismetTextLibrary.Conv_TextToString` (`|FormatText` "Created {category} settings! \nCount: {b}" _categoryname (`KismetArrayLibrary.Array_Length` `Settings Groups`))))
      (bind _modloadermanagerinstance (`/PDML/Blueprints/Utilities/BPFL_ModLoader.GetModLoaderManager` null))
      (`KismetArrayLibrary.Array_AddUnique` (`/PDML/Blueprints/BP_ModLoader.ModSettingsConfig` _modloadermanagerinstance) (make `SBZSettingsMenuCategoryInfo` (`KismetTextLibrary.Conv_NameToText` ModName) false "" false "" _categoryname "/Script/Starbreeze.SBZSettingsFunctions" `Settings Groups`))
      (return true))))

(fn `CreateSettingsGroup`
  (params (ModName :type Name) (GroupID :type Name) (GroupName :type Name) (SettingsData :type "Array of SBZSettingData Structure"))
  (returns (Array :type "Array of SBZSettingsMenuGroupInfo Structure"))
  (return (`|MakeArray` (make `SBZSettingsMenuGroupInfo` (`KismetTextLibrary.Conv_NameToText` GroupName) false "" false "" (`KismetStringLibrary.Conv_StringToName` (`KismetTextLibrary.Conv_TextToString` (`|FormatText` "Settings_{ModName}_{Group}" ModName GroupID))) false false SettingsData))))

(fn `CreateStringSetting`
  (params (UniqueName :type Name) (`Display Text` :type Text) (`Apply Change Immediately` :type Boolean) (`Get Default Value Function Name` :type Name) (`Get Value Function Name` :type Name) (`Set Value Function Name` :type Name) (`String Value` :type String))
  (returns (SBZSettingData :type "SBZSettingData Structure"))
  (return (make `SBZSettingData` `Display Text` false "" false "" UniqueName "" "StringControl" "None" "" `Apply Change Immediately` false true "GetButtonVisibilityAlways" false false false "" "None" `Get Default Value Function Name` `Get Value Function Name` `Set Value Function Name` "GetDefaultPrimaryKeyboardBinding" "GetPrimaryKeyboardBinding" "SetPrimaryKeyboardBinding" "GetDefaultSecondaryKeyboardBinding" "GetSecondaryKeyboardBinding" "SetSecondaryKeyboardBinding" true true "" "" false false "" 0 0 0.0 0.0 0.0 0.0 0.0 `String Value`)))

(fn `CreateToggleSetting`
  (params (UniqueName :type Name) (`Display Text` :type Text) (`Apply Change Immediately` :type Boolean) (`Get Default Value Function Name` :type Name) (`Get Value Function Name` :type Name) (`Set Value Function Name` :type Name) (`Bool Value` :type Boolean))
  (returns (SBZSettingData :type "SBZSettingData Structure"))
  (return (make `SBZSettingData` `Display Text` false "" false "" UniqueName "" "Toggle" "None" "" `Apply Change Immediately` false true "GetButtonVisibilityAlways" false false false "" "None" `Get Default Value Function Name` `Get Value Function Name` `Set Value Function Name` "GetDefaultPrimaryKeyboardBinding" "GetPrimaryKeyboardBinding" "SetPrimaryKeyboardBinding" "GetDefaultSecondaryKeyboardBinding" "GetSecondaryKeyboardBinding" "SetSecondaryKeyboardBinding" true true "" "" `Bool Value` `Bool Value`)))

(fn `DoesCategoryAlreadyExist`
  (params (CategoryName :type Name))
  (returns (bExists :type Boolean))
  (locals (bFound :type Boolean))
  (bind _modloadermanagerinstance (`/PDML/Blueprints/Utilities/BPFL_ModLoader.GetModLoaderManager` null))
  (for _array_element (`/PDML/Blueprints/BP_ModLoader.ModSettingsConfig` _modloadermanagerinstance)
    (if (== (`.CategoryName` (break `SBZSettingsMenuCategoryInfo` _array_element)) CategoryName)
      (set `local.bFound` true)
      (break)))
  (return (`local.bFound`)))

(fn `GetCategoryNameFromModName`
  (params (ModName :type Name))
  (returns (CategoryName :type Name))
  (return (`KismetStringLibrary.Conv_StringToName` (`KismetTextLibrary.Conv_TextToString` (`|FormatText` "Settings_{ModName}_Category" ModName)))))

(fn `GetColorSettingValue`
  (params (ConfigName :type String) (UniqueName :type "Name (by ref)"))
  (returns (Value :type "LinearColor Structure") (Successful :type Boolean))
  (bind _config (`self.LoadConfig` ConfigName))
  (bind (_value _returnvalue) (`BlueprintMapLibrary.Map_Find` (`/PDML/Blueprints/SaveGame/SaveGame_PDML_Settings.ColorMap` _config) UniqueName))
  (return _value _returnvalue))

(fn `GetFloatSettingValue`
  (params (ConfigName :type String) (UniqueName :type "Name (by ref)"))
  (returns (Value :type "Float (double-precision)") (Successful :type Boolean))
  (bind _config (`self.LoadConfig` ConfigName))
  (bind (_value _returnvalue) (`BlueprintMapLibrary.Map_Find` (`/PDML/Blueprints/SaveGame/SaveGame_PDML_Settings.FloatMap` _config) UniqueName))
  (return _value _returnvalue))

(fn `GetKeybindSettingValue`
  (params (ConfigName :type String) (UniqueName :type "Name (by ref)"))
  (returns (PrimaryKeybind :type "InputChord Structure") (SecondaryKeybind :type "InputChord Structure") (PrimarySuccessful :type Boolean) (SecondarySuccessful :type Boolean))
  (bind _config (`self.LoadConfig` ConfigName))
  (bind (_value _returnvalue) (`BlueprintMapLibrary.Map_Find` (`/PDML/Blueprints/SaveGame/SaveGame_PDML_Settings.PrimaryKeybindMap` _config) UniqueName))
  (bind (_value_2 _returnvalue_2) (`BlueprintMapLibrary.Map_Find` (`/PDML/Blueprints/SaveGame/SaveGame_PDML_Settings.SecondaryKeybindMap` _config) UniqueName))
  (return _value _value_2 _returnvalue _returnvalue_2))

(fn `GetModNameFromCategoryName`
  (params (CategoryName :type Name))
  (returns (ModName :type Name))
  (return (`KismetStringLibrary.Conv_StringToName` (`KismetStringLibrary.Split` (`.RightS` (`KismetStringLibrary.Split` (`KismetStringLibrary.Conv_NameToString` CategoryName) "Settings_")) "_Category"))))

(fn `GetStringSettingValue`
  (params (ConfigName :type String) (UniqueName :type "Name (by ref)"))
  (returns (Value :type String) (Successful :type Boolean))
  (bind _config (`self.LoadConfig` ConfigName))
  (bind (_value _returnvalue) (`BlueprintMapLibrary.Map_Find` (`/PDML/Blueprints/SaveGame/SaveGame_PDML_Settings.StringMap` _config) UniqueName))
  (return _value _returnvalue))

(fn `GetToggleSettingValue`
  (params (ConfigName :type String) (UniqueName :type "Name (by ref)"))
  (returns (Value :type Boolean) (Successful :type Boolean))
  (bind _config (`self.LoadConfig` ConfigName))
  (bind (_value _returnvalue) (`BlueprintMapLibrary.Map_Find` (`/PDML/Blueprints/SaveGame/SaveGame_PDML_Settings.ToggleMap` _config) UniqueName))
  (return _value _returnvalue))

(fn `IsChordDown`
  (params (Target :type "PlayerController Object Reference") (Chord :type "InputChord Structure"))
  (returns (bIsDown :type Boolean))
  (return (`PlayerController.IsInputKeyDown` Target (`.Key` (break `InputChord` Chord)))))

(fn `LoadConfig`
  (params (ConfigName :type String))
  (returns (Config :type "/PDML/Blueprints/SaveGame/SaveGame_PDML_Settings Object Reference") (FirstTime :type Boolean) (Successful :type Boolean))
  (bind _returnvalue (`GameplayStatics.DoesSaveGameExist` ConfigName))
  (if _returnvalue
    (bind _returnvalue_2 (`GameplayStatics.LoadGameFromSlot` ConfigName))
    (bind _assave_game_pdml_settings (cast `/PDML/Blueprints/SaveGame/SaveGame_PDML_Settings` _returnvalue_2)
      (:`then`
        (return _assave_game_pdml_settings false true))
      (:`CastFailed`
        (return null false false)))
    (else
      (bind _returnvalue_3 (`GameplayStatics.CreateSaveGameObject` "/PDML/Blueprints/SaveGame/SaveGame_PDML_Settings.SaveGame_PDML_Settings_C"))
      (bind (_config _successful) (`self.SaveConfig` _returnvalue_3 ConfigName))
      (return _config true _successful))))

(fn `RemoveSettingsCategory`
  (params (ModName :type Name))
  (returns (Successful :type Boolean))
  (locals (bRemoved :type Boolean :default false))
  (bind _categoryname (`self.GetCategoryNameFromModName` ModName))
  (bind _bexists (`self.DoesCategoryAlreadyExist` _categoryname))
  (if _bexists
    (bind _modloadermanagerinstance (`/PDML/Blueprints/Utilities/BPFL_ModLoader.GetModLoaderManager` null))
    (bind _modsettingsconfig (`/PDML/Blueprints/BP_ModLoader.ModSettingsConfig` _modloadermanagerinstance))
    (for _array_element _modsettingsconfig
      (if (== (`.CategoryName` (break `SBZSettingsMenuCategoryInfo` _array_element)) _categoryname)
        (bind _returnvalue (`KismetArrayLibrary.Array_RemoveItem` _modsettingsconfig _array_element))
        (set `local.bRemoved` _returnvalue)
        (break)))
    (return (`local.bRemoved`))))

(fn `SaveConfig`
  (params (SaveGameObject :type "/PDML/Blueprints/SaveGame/SaveGame_PDML_Settings Object Reference") (ConfigName :type String))
  (returns (Config :type "/PDML/Blueprints/SaveGame/SaveGame_PDML_Settings Object Reference") (Successful :type Boolean))
  (bind _returnvalue (`GameplayStatics.SaveGameToSlot` SaveGameObject ConfigName))
  (return SaveGameObject _returnvalue))

(fn `SetColorSettingValue`
  (params (ConfigName :type String) (UniqueName :type "Name (by ref)") (Value :type "LinearColor Structure (by ref)"))
  (bind _config (`self.LoadConfig` ConfigName))
  (`BlueprintMapLibrary.Map_Add` (`/PDML/Blueprints/SaveGame/SaveGame_PDML_Settings.ColorMap` _config) UniqueName Value)
  (`self.SaveConfig` _config ConfigName))

(fn `SetFloatSettingValue`
  (params (ConfigName :type String) (UniqueName :type "Name (by ref)") (Value :type "Float (double-precision) (by ref)"))
  (bind _config (`self.LoadConfig` ConfigName))
  (`BlueprintMapLibrary.Map_Add` (`/PDML/Blueprints/SaveGame/SaveGame_PDML_Settings.FloatMap` _config) UniqueName Value)
  (`self.SaveConfig` _config ConfigName))

(fn `SetKeybindSettingValue`
  (params (ConfigName :type String) (UniqueName :type "Name (by ref)") (PrimaryBinding :type "InputChord Structure (by ref)") (SecondaryBinding :type "InputChord Structure"))
  (bind _config (`self.LoadConfig` ConfigName))
  (`BlueprintMapLibrary.Map_Add` (`/PDML/Blueprints/SaveGame/SaveGame_PDML_Settings.PrimaryKeybindMap` _config) UniqueName PrimaryBinding)
  (`BlueprintMapLibrary.Map_Add` (`/PDML/Blueprints/SaveGame/SaveGame_PDML_Settings.SecondaryKeybindMap` _config) UniqueName SecondaryBinding)
  (`self.SaveConfig` _config ConfigName))

(fn `SetStringSetting`
  (params (ConfigName :type String) (UniqueName :type "Name (by ref)") (Value :type "String (by ref)"))
  (bind _config (`self.LoadConfig` ConfigName))
  (`BlueprintMapLibrary.Map_Add` (`/PDML/Blueprints/SaveGame/SaveGame_PDML_Settings.StringMap` _config) UniqueName Value)
  (`self.SaveConfig` _config ConfigName))

(fn `SetToggleSettingValue`
  (params (ConfigName :type String) (UniqueName :type "Name (by ref)") (Value :type "Boolean (by ref)"))
  (bind _config (`self.LoadConfig` ConfigName))
  (`BlueprintMapLibrary.Map_Add` (`/PDML/Blueprints/SaveGame/SaveGame_PDML_Settings.ToggleMap` _config) UniqueName Value)
  (`self.SaveConfig` _config ConfigName))